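; First-person player character for a Superliminal-style forced-perspective mechanic that picks up, rotates and drops BP_Moveable objects.
; A looping timer line-traces from the camera to drive crosshair hover.
; Pickup lerps the object to view center, then opens a Tick gate that steps scaled box traces outward to the first hit, scaling the object proportionally to distance.
; Shift and Ctrl select the rotation axis, and a teleport helper rescales player size, movement and reach.
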(event Custom|LerpLocation
  (params (StartLocation :type Vector))
  (bind _alpha (Timeline|TL_Lerp Play)
    (:Update
      (Transformation|SetRelativeLocation (Variables|Default|GetHeldObject) (Math|Vector|Lerp(Vector) StartLocation (* (Math|Vector|Distance(Vector) "0, 0, 0" StartLocation) "1.000000,0.000000,0.000000") _alpha) false true))
    (:Finished
      (CallFunction|CEOpenGate))))

(event Custom|CE_OpenGate
  (bind _heldobject (Variables|Default|GetHeldObject))
  (Utilities|FlowControl|Gate true) ; enters at Open
)

(event Custom|CE_CloseGate
  (bind _heldobject (Variables|Default|GetHeldObject))
  (Utilities|FlowControl|Gate true) ; enters at Close
)

(event Input|EnhancedActionEvents|EnhancedInputActionIA_Interact
  (params (ActionValue :type Boolean) (ElapsedSeconds :type Float%20%28double-precision%29) (TriggeredSeconds :type Float%20%28double-precision%29) (InputAction :type Input%20Action%20Object%20Reference :default "/Game/Superliminal/Inputs/IA_Interact.IA_Interact"))
  (Variables|Default|GetHeldObject
    (:then
      (CallFunction|DropObject))
    (:else
      (CallFunction|PickUpObject))))

(event Input|EnhancedActionEvents|EnhancedInputActionIA_Rotate
  (params (ActionValue :type Float%20%28double-precision%29) (ElapsedSeconds :type Float%20%28double-precision%29) (TriggeredSeconds :type Float%20%28double-precision%29) (InputAction :type Input%20Action%20Object%20Reference :default "/Game/Superliminal/Inputs/IA_Rotate.IA_Rotate"))
  (|RotateObject (* ActionValue 7.2)))

(event EventBeginPlay
  (|CallParentFunction)
  (Input|AddMappingContext (PlayerController|LocalPlayerSubsystems|GetEnhancedInputLocalPlayerSubsystem (Game|GetPlayerController 0)) "/Game/Superliminal/Inputs/IMC_Superliminal.IMC_Superliminal" 0 "(bIgnoreAllPressedKeysUntilRelease=True,bForceImmediately=False,bNotifyUserSettings=False)")
  (bind _returnvalue (UserInterface|CreateWidget "/Game/Superliminal/UI/UMG_Crosshair.UMG_Crosshair_C"))
  (bind _output_get (Variables|Default|SetAsUMGCrosshair _returnvalue))
  (UserInterface|Viewport|AddtoViewport _output_get 0)
  (bind _returnvalue_2 (Utilities|Time|SetTimerbyFunctionName 0 "TraceValidTarget" 0.05 true))
  (Variables|Default|SetCrosshairTime _returnvalue_2))

(event EventTick
  (params (DeltaSeconds :type Float%20%28single-precision%29))
  (bind _heldobject (Variables|Default|GetHeldObject))
  (Utilities|FlowControl|Gate true
    (:Exit
      (bind (_newlocation _scalemodifier) (CallFunction|CustomBoxTrace (Variables|Default|GetInitialBounds) (Variables|Default|GetInitialDistance)))
      (Transformation|SetWorldLocation _heldobject _newlocation false false)
      (Transformation|SetWorldScale3D _heldobject (* _scalemodifier (Variables|Default|GetInitialScale))))))

(event Input|KeyboardEvents|LeftShift
  (params (Key :type Key%20Structure :default "None"))
  (:Pressed
    (Variables|Default|SetShiftIsHeld true))
  (:Released
    (Variables|Default|SetShiftIsHeld false)))

(event Input|KeyboardEvents|LeftCtrl
  (params (Key :type Key%20Structure :default "None"))
  (:Pressed
    (Variables|Default|SetCtrlIsHeld true))
  (:Released
    (Variables|Default|SetCtrlIsHeld false)))

(fn ConstructionScript
  (|CallParentFunction))

(fn TraceValidTarget
  (bind (_outhit _didhitsomething) (CallFunction|LineTracefromCamera))
  (if _didhitsomething
    (bind _asbp_moveable (Utilities|Casting|CastToBP_Moveable (.HitActor (Collision|BreakHitResult _outhit)))
      (:then
        (if (not (Variables|/Game/Superliminal/Blueprints/Movable/BP_Moveable.BP_Moveable_C|GetIsLocked _asbp_moveable))
          (if (not (Variables|/Game/Superliminal/UI/UMG_Crosshair.UMG_Crosshair_C|GetIsHover (Variables|Default|GetAsUMGCrosshair)))
            (Default|Hover (Variables|Default|GetAsUMGCrosshair)))
          (else
            (if (Variables|/Game/Superliminal/UI/UMG_Crosshair.UMG_Crosshair_C|GetIsHover (Variables|Default|GetAsUMGCrosshair)) :!label _label
              (Default|Unhover (Variables|Default|GetAsUMGCrosshair))))))
      (:CastFailed
        (goto _label)))))

(fn LineTracefromCamera
  (bind _firstpersoncamera (Variables|Default|GetFirstPersonCamera))
  (bind _returnvalue (Transformation|GetWorldLocation _firstpersoncamera))
  (bind (_outhit _returnvalue_2) (Collision|LineTraceByChannel _returnvalue (+ _returnvalue (* (Math|Vector|GetForwardVector _firstpersoncamera) (Variables|Default|GetMaxRange))) "TraceTypeQuery1" false 0 "None"))
  (return _outhit _returnvalue_2))

(fn PickUpObject
  (bind (_outhit _didhitsomething) (CallFunction|LineTracefromCamera))
  (if _didhitsomething
    (bind _asbp_moveable (Utilities|Casting|CastToBP_Moveable (.HitActor (Collision|BreakHitResult _outhit))))
    (bind _didpickitup (Default|SelfPickup _asbp_moveable (Variables|Default|GetFirstPersonCamera)))
    (if _didpickitup
      (bind _output_get (Variables|Default|SetHeldObject (Variables|/Game/Superliminal/Blueprints/Movable/BP_Moveable.BP_Moveable_C|GetStaticMesh _asbp_moveable)))
      (CallFunction|LerpLocation (Variables|/Script/Engine.SceneComponent|GetRelativeLocation _output_get))
      (Utilities|Time|ClearandInvalidateTimerbyHandle (Variables|Default|GetCrosshairTime))
      (Default|Hover (Variables|Default|GetAsUMGCrosshair))
      (Variables|Default|SetInitialBounds (.BoxExtent (Collision|GetComponentBounds (Variables|Default|GetHeldObject))))
      (Variables|Default|SetInitialDistance (Math|Vector|Distance(Vector) "0, 0, 0" (Variables|/Script/Engine.SceneComponent|GetRelativeLocation (Variables|Default|GetHeldObject))))
      (Variables|Default|SetInitialScale (Transformation|GetWorldScale (Variables|Default|GetHeldObject))))))

(fn DropObject
  (bind _heldobject (Variables|Default|GetHeldObject)
    (:then
      (bind _asbp_moveable (Utilities|Casting|CastToBP_Moveable (Components|GetOwner _heldobject)))
      (Default|SelfDrop _asbp_moveable)
      (Variables|Default|SetHeldObject 0)
      (Default|Unhover (Variables|Default|GetAsUMGCrosshair))
      (bind _returnvalue (Utilities|Time|SetTimerbyFunctionName 0 "TraceValidTarget" 0.05 true))
      (Variables|Default|SetCrosshairTime _returnvalue)
      (CallFunction|CECloseGate))
    (:else)))

(fn CustomBoxTrace
  (params (InitialBounds :type Vector) (InitialDistance :type Float%20%28double-precision%29))
  (bind _firstpersoncamera (Variables|Default|GetFirstPersonCamera))
  (LocalVariables|SetLCurrentBounds InitialBounds)
  (for _index (range 10 (Math|Float|Truncate (/ (Variables|Default|GetMaxRange) 5.0)))
    (LocalVariables|SetLCurrentDistance (Math|Conversions|ToFloat(Integer) (* _index 5)))
    (LocalVariables|SetLCurrentBounds (* (Variables|Default|GetInitialBounds) (/ (LocalVariables|GetLCurrentDistance) (Variables|Default|GetInitialDistance))))
    (LocalVariables|SetLLocation (+ (Transformation|GetWorldLocation _firstpersoncamera) (* (Math|Vector|GetForwardVector _firstpersoncamera) (LocalVariables|GetLCurrentDistance))))
    (bind _returnvalue (Collision|BoxTraceByChannel (LocalVariables|GetLLocation) (LocalVariables|GetLLocation) (* (LocalVariables|GetLCurrentBounds) 1.4) "0, 0, 0" "TraceTypeQuery1" false 0 "None"))
    (if _returnvalue
      (return (LocalVariables|GetLLocation) (/ (LocalVariables|GetLCurrentDistance) (Variables|Default|GetInitialDistance)))))
  (return (LocalVariables|GetLLocation) (/ (LocalVariables|GetLCurrentDistance) (Variables|Default|GetInitialDistance))))

(fn ResizePlayerAfterTeleport
  (params (NewSize :type Float%20%28double-precision%29))
  (bind _charactermovement (Variables|Character|GetCharacterMovement))
  (Transformation|SetActorScale3D (* (Transformation|GetActorScale3D) NewSize))
  (Variables|/Script/Engine.CharacterMovementComponent|SetMaxWalkSpeed _charactermovement (* (Variables|/Script/Engine.CharacterMovementComponent|GetMaxWalkSpeed _charactermovement) NewSize))
  (Variables|/Script/Engine.CharacterMovementComponent|SetJumpZVelocity _charactermovement (* (Variables|/Script/Engine.CharacterMovementComponent|GetJumpZVelocity _charactermovement) NewSize))
  (Variables|/Script/Engine.CharacterMovementComponent|SetGravityScale _charactermovement (* (Variables|/Script/Engine.CharacterMovementComponent|GetGravityScale _charactermovement) NewSize))
  (Variables|Default|SetMaxRange (* (Variables|Default|GetMaxRange) NewSize)))