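; Superliminal-style perspective puzzle that hides a target actor behind its projected image until the player's camera matches the capture viewpoint.
; On BeginPlay, scene captures photograph and mask the target, repeating in dark mode.
; Box traces over distance-sorted ProjectOn actors spawn M_Projection decals, each masked by a capture of nearer actors.
; Tick checks camera alignment, then reveals the target, unlocks physics if it is BP_Moveable, and destroys itself.
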(event EventBeginPlay
  (bind _projectiontarget (Variables|Default|GetProjectionTarget))
  (CallFunction|ProjectItem)
  (if (Variables|Default|GetDarkModeOn)
    (for _index (range 0 (Variables|Default|GetDarkModeIterations))
      (CallFunction|ProjectItem)))
  (Rendering|SetActorHiddenInGame _projectiontarget true)
  (Collision|SetActorEnableCollision _projectiontarget true))

(event Collision|EventActorBeginOverlap
  (params (OtherActor :type Actor%20Object%20Reference)))

(event EventTick
  (params (DeltaSeconds :type Float%20%28single-precision%29))
  (bind _isinposition (CallFunction|IsPlayerinPosition))
  (if _isinposition
    (CallFunction|FreeActor)))

(fn ConstructionScript)

(fn ProjectItem
  ;[1 1 1] Setup the SceneCapture Component to look straight at capture target
  (Transformation|SetWorldRotation (Variables|Default|GetSceneCaptureComponent2D) (Math|Rotator|FindLookatRotation (Transformation|GetWorldLocation (Variables|Default|GetSceneCaptureComponent2D)) (Transformation|GetActorLocation (Variables|Default|GetProjectionTarget))) false false)
  (Utilities|Array|Add (Variables|/Script/Engine.SceneCaptureComponent|GetShowOnlyActors (Variables|Default|GetSceneCaptureComponent2D)) (Variables|Default|GetProjectionTarget))
  (Utilities|Array|Add (Variables|/Script/Engine.SceneCaptureComponent|GetShowOnlyActors (Variables|Default|GetSceneCaptureComponent2DMask)) (Variables|Default|GetProjectionTarget))
  (Utilities|FlowControl|Sequence
    (:then_0
      ;[1 1 1] CapturePhoto
      (bind _returnvalue (Rendering|CreateRenderTarget2D 2048 2048 "RTF_RGBA16f"))
      (Variables|/Script/Engine.SceneCaptureComponent2D|SetTextureTarget (Variables|Default|GetSceneCaptureComponent2D) _returnvalue)
      (Rendering|SceneCapture|CaptureScene (Variables|Default|GetSceneCaptureComponent2D) :!class /Script/Engine.SceneCaptureComponent2D))
    (:then_1
      (bind _returnvalue_2 (Rendering|CreateRenderTarget2D 1024 1024 "RTF_RGBA16f"))
      (Variables|/Script/Engine.SceneCaptureComponent2D|SetTextureTarget (Variables|Default|GetSceneCaptureComponent2DMask) _returnvalue_2)
      (Rendering|SceneCapture|CaptureScene (Variables|Default|GetSceneCaptureComponent2DMask) :!class /Script/Engine.SceneCaptureComponent2D))
    (:then_2
      (CallFunction|SortbyDistance))
    (:then_3
      (CallFunction|TraceforProjection))))

(fn SortbyDistance
  (for _index (range 0 (Utilities|Array|LastIndex (Variables|Default|GetProjectOn)))
    (bind _output_get (LocalVariables|SetLIndexA _index))
    (LocalVariables|SetLActorA (Utilities|Array|Get(acopy) (Variables|Default|GetProjectOn) _output_get))
    (for _index_2 (range (LocalVariables|GetLIndexA) (Utilities|Array|LastIndex (Variables|Default|GetProjectOn)))
      (bind _output_get_2 (LocalVariables|SetLIndexB _index_2))
      (LocalVariables|SetLActorB (Utilities|Array|Get(acopy) (Variables|Default|GetProjectOn) _output_get_2))
      (if (< (Transformation|GetDistanceTo (LocalVariables|GetLActorB)) (Transformation|GetDistanceTo (LocalVariables|GetLActorA)))
        (Utilities|Array|Swap (Variables|Default|GetProjectOn) (LocalVariables|GetLIndexA) (LocalVariables|GetLIndexB))))))

(fn TraceforProjection
  (bind (_start _end _halfsize _orientation) (CallFunction|BoxTraceInfo))
  (bind (_start_2 _end_2 _halfsize_2 _orientation_2) (CallFunction|BoxTraceInfo))
  (bind _outhits (Class|KismetSystemLibrary|BoxTraceMulti _start _end _halfsize _orientation "TraceTypeQuery1" false (Variables|Default|GetProjectOn) "None" true))
  (for _array_element _outhits
    (Utilities|Array|AddUnique (LocalVariables|GetLIgnore) (.HitActor (Collision|BreakHitResult _array_element))))
  (for _array_element_2 (Variables|Default|GetProjectOn)
    (LocalVariables|SetLCurrentTarget _array_element_2)
    (bind _outhit (Collision|BoxTraceByChannel _start_2 _end_2 _halfsize_2 _orientation_2 "TraceTypeQuery1" false (LocalVariables|GetLIgnore) "None"))
    (Utilities|FlowControl|Sequence
      (:then_0
        (bind _asstatic_mesh_component (Utilities|Casting|CastToStaticMeshComponent (.HitComponent (Collision|BreakHitResult _outhit))))
        (bind _returnvalue (AddComponent|AddDecalComponent true (Math|Transform|MakeTransform (+ (* (Math|Vector|Normalize (- (.TraceStart (Collision|BreakHitResult _outhit)) (.TraceEnd (Collision|BreakHitResult _outhit)))) 5.1) (/ (+ (Math|Transform|TransformLocation (Transformation|GetActorTransform (Components|GetOwner _asstatic_mesh_component)) (.Min (Components|StaticMesh|GetLocalBounds _asstatic_mesh_component))) (Math|Transform|TransformLocation (Transformation|GetActorTransform (Components|GetOwner _asstatic_mesh_component)) (.Max (Components|StaticMesh|GetLocalBounds _asstatic_mesh_component)))) 2.0)) (Transformation|GetWorldRotation _asstatic_mesh_component) "1.000000,1.000000,1.000000")))
        (bind _output_get (LocalVariables|SetLDecal _returnvalue))
        (Transformation|SetWorldScale3D _output_get (+ (* (.Max (Components|StaticMesh|GetLocalBounds _asstatic_mesh_component)) (Transformation|GetWorldScale _asstatic_mesh_component)) 5.0))
        (bind _returnvalue_2 (Rendering|CreateRenderTarget2D 2048 2048 "RTF_RGBA16f"))
        (bind _returnvalue_3 (AddComponent|AddSceneCaptureComponent2D false (Transformation|GetRelativeTransform (Variables|Default|GetSceneCaptureComponent2D))))
        (Variables|/Script/Engine.SceneCaptureComponent2D|SetTextureTarget _returnvalue_3 _returnvalue_2)
        (Utilities|Array|AppendArray (Variables|/Script/Engine.SceneCaptureComponent|GetShowOnlyActors _returnvalue_3) (LocalVariables|GetLShowOnly))
        (Rendering|SceneCapture|CaptureScene _returnvalue_3 :!class /Script/Engine.SceneCaptureComponent2D)
        (bind _returnvalue_4 (Rendering|Material|CreateDynamicMaterialInstance "/Game/Superliminal/Assets/Materials/M_Projection.M_Projection" "None" "None" :!class /Script/Engine.KismetMaterialLibrary))
        (Rendering|Components|Decal|SetDecalMaterial (LocalVariables|GetLDecal) _returnvalue_4)
        (CallFunction|UpdateMaterialParams _returnvalue_4 _returnvalue_2))
      (:then_1
        (Utilities|Array|Add (LocalVariables|GetLShowOnly) (LocalVariables|GetLCurrentTarget))
        (Utilities|Array|Add (LocalVariables|GetLIgnore) (LocalVariables|GetLCurrentTarget))))))

(fn IsPlayerinPosition
  (bind _returnvalue (Game|GetPlayerCameraManager 0))
  (return (and (Utilities|Operators|EqualEqual (Transformation|GetWorldLocation (Variables|Default|GetSceneCaptureComponent2D)) (Transformation|GetActorLocation _returnvalue) 1e+01) (Utilities|Operators|EqualEqual (Transformation|GetWorldRotation (Variables|Default|GetSceneCaptureComponent2D)) (Transformation|GetActorRotation _returnvalue) 4.0))))

(fn FreeActor
  (bind _projectiontarget (Variables|Default|GetProjectionTarget))
  (Rendering|SetActorHiddenInGame _projectiontarget false)
  (Collision|SetActorEnableCollision _projectiontarget true)
  (bind _asbp_moveable (Utilities|Casting|CastToBP_Moveable (Variables|Default|GetProjectionTarget))
    (:then
      (Variables|/Game/Superliminal/Blueprints/Movable/BP_Moveable.BP_Moveable_C|SetIsLocked _asbp_moveable false)
      (Physics|SetSimulatePhysics (Variables|/Game/Superliminal/Blueprints/Movable/BP_Moveable.BP_Moveable_C|GetStaticMesh _asbp_moveable) true)
      (Actor|DestroyActor))
    (:CastFailed
      (Actor|DestroyActor))))

(fn BoxTraceInfo
  (bind _returnvalue (Transformation|GetActorLocation))
  (return _returnvalue (+ _returnvalue (* (Math|Vector|GetForwardVector (Variables|Default|GetSceneCaptureComponent2D)) 5e+03)) "256.000000,256.000000,256.000000" (Transformation|GetWorldRotation (Variables|Default|GetSceneCaptureComponent2D))))

(fn UpdateMaterialParams
  (params (Material :type Material%20Instance%20Dynamic%20Object%20Reference) (TextureTarget :type Texture%20Render%20Target%202D%20Object%20Reference))
  (Rendering|Material|SetVectorParameterValue Material "Location" (Math|Conversions|ToLinearColor(Vector) (Transformation|GetWorldLocation (Variables|Default|GetSceneCaptureComponent2D))) :!class /Script/Engine.MaterialInstanceDynamic)
  (Rendering|Material|SetVectorParameterValue Material "RightVector" (Math|Conversions|ToLinearColor(Vector) (Math|Vector|GetRightVector (Variables|Default|GetSceneCaptureComponent2D))) :!class /Script/Engine.MaterialInstanceDynamic)
  (Rendering|Material|SetVectorParameterValue Material "UpVector" (Math|Conversions|ToLinearColor(Vector) (Math|Vector|GetUpVector (Variables|Default|GetSceneCaptureComponent2D))) :!class /Script/Engine.MaterialInstanceDynamic)
  (Rendering|Material|SetVectorParameterValue Material "ForwardVector" (Math|Conversions|ToLinearColor(Vector) (Math|Vector|GetForwardVector (Variables|Default|GetSceneCaptureComponent2D))) :!class /Script/Engine.MaterialInstanceDynamic)
  (Rendering|Material|SetScalarParameterValue Material "FOV" (Variables|/Script/Engine.SceneCaptureComponent2D|GetFOVAngle (Variables|Default|GetSceneCaptureComponent2D)) :!class /Script/Engine.MaterialInstanceDynamic)
  (Rendering|Material|SetTextureParameterValue Material "ProjectedTexture" (Variables|/Script/Engine.SceneCaptureComponent2D|GetTextureTarget (Variables|Default|GetSceneCaptureComponent2D)))
  (Rendering|Material|SetTextureParameterValue Material "ProjectedMask" TextureTarget)
  (Rendering|Material|SetTextureParameterValue Material "ProjectedActorMask" (Variables|/Script/Engine.SceneCaptureComponent2D|GetTextureTarget (Variables|Default|GetSceneCaptureComponent2DMask))))