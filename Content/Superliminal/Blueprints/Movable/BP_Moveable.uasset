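; BP_Moveable is a movable prop in the Superliminal game folder that another component can pick up and drop.
; SelfPickup refuses when IsLocked; otherwise it attaches the mesh to the given component, turns off physics and collision, sets IsHeld and reports success.
; SelfDrop detaches the mesh in place and restores physics and collision.
; Locked props also have physics simulation turned off at BeginPlay.
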(event EventBeginPlay
  (if (Variables|Default|GetIsLocked)
    (Physics|SetSimulatePhysics (Variables|Default|GetStaticMesh) false)))

(event Collision|EventActorBeginOverlap
  (params (OtherActor :type Actor%20Object%20Reference)))

(event EventTick
  (params (DeltaSeconds :type Float%20%28single-precision%29)))

(fn ConstructionScript)

(fn SelfDrop
  (bind _staticmesh (Variables|Default|GetStaticMesh))
  (Transformation|DetachFromComponent (Variables|Default|GetStaticMesh) "KeepWorld" "KeepWorld" "KeepWorld" true)
  (Physics|SetSimulatePhysics _staticmesh true)
  (Collision|SetCollisionEnabled _staticmesh "QueryAndPhysics")
  (Variables|Default|SetIsHeld false))

(fn SelfPickup
  (params (ParentComponent :type Scene%20Component%20Object%20Reference))
  (bind _staticmesh (Variables|Default|GetStaticMesh))
  (if (Variables|Default|GetIsLocked)
    (return false)
    (else
      (Transformation|AttachComponentToComponent (Variables|Default|GetStaticMesh) ParentComponent "None" "KeepWorld" "KeepWorld" "KeepWorld" true)
      (Physics|SetSimulatePhysics _staticmesh false)
      (Collision|SetCollisionEnabled _staticmesh "NoCollision")
      (Variables|Default|SetIsHeld true)
      (return true))))