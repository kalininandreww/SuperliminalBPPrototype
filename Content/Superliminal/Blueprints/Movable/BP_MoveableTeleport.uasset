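; Movable portal that pairs with a linked portal to show a see-through view and teleport the Superliminal character, resizing them by the portals' scale ratio.
; The primary links both render targets at construction; on Tick, enabled portals position the linked scene capture relative to the player camera, resize the target and set a clip plane.
; Front-side overlap while not held drops the player's object and triggers teleportation, remapping location, control rotation and velocity.
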(event OnComponentBeginOverlap(DropHeld)
  (params (OverlappedComponent :type Primitive%20Component%20Object%20Reference) (OtherActor :type Actor%20Object%20Reference) (OtherComp :type Primitive%20Component%20Object%20Reference) (OtherBodyIndex :type Integer) (bFromSweep :type Boolean) (SweepResult :type Hit%20Result%20Structure%20%28by%20ref%29))
  (if (not (Variables|Default|GetIsHeld))
    (bind _asbp_superliminal_character (Utilities|Casting|CastToBP_SuperliminalCharacter OtherActor))
    (Default|DropObject _asbp_superliminal_character)
    (if (CallFunction|IsPlayerInfront)
      (Variables|Default|SetStartOverlap true))))

(event OnComponentEndOverlap(DropHeld)
  (params (OverlappedComponent :type Primitive%20Component%20Object%20Reference) (OtherActor :type Actor%20Object%20Reference) (OtherComp :type Primitive%20Component%20Object%20Reference) (OtherBodyIndex :type Integer))
  (Utilities|Casting|CastToBP_SuperliminalCharacter OtherActor)
  (Variables|Default|SetStartOverlap false))

(event EventBeginPlay
  (|CallParentFunction)
  (bind _asbp_superliminal_character (Utilities|Casting|CastToBP_SuperliminalCharacter (Game|GetPlayerCharacter 0)))
  (Variables|Default|SetAs%20BP%20Superliminal%20Character _asbp_superliminal_character))

(event Collision|EventActorBeginOverlap
  (params (OtherActor :type Actor%20Object%20Reference))
  (|CallParentFunction OtherActor) ; This node is disabled and will not be called.\nDrag off pins to build functionality.
)

(event EventTick
  (params (DeltaSeconds :type Float%20%28single-precision%29))
  (|CallParentFunction DeltaSeconds)
  (if (Variables|Default|GetIsEnabled)
    (CallFunction|UpdateRenerTarget)))

(fn ConstructionScript
  (|CallParentFunction)
  (CallFunction|SetupLink))

(fn SetupLink
  (if (and (Variables|Default|GetIsEnabled) (Variables|Default|GetIsPrimary))
    (CallFunction|SetupRenderTarget "/Game/Superliminal/Assets/Materials/RenderTargets/RT_Portal0.RT_Portal0")
    (Variables|BP_MoveableTeleport_C|SetLinkedPortal (Variables|Default|GetLinkedPortal) self)
    (CallFunction|SetupRenderTarget (Variables|Default|GetLinkedPortal) "/Game/Superliminal/Assets/Materials/RenderTargets/RT_Portal1.RT_Portal1")))

(fn SetupRenderTarget
  (params (RenderTarget :type Texture%20Render%20Target%202D%20Object%20Reference))
  (Variables|/Script/Engine.SceneCaptureComponent2D|SetTextureTarget (Variables|Default|GetSceneCaptureComponent2D) RenderTarget)
  (Rendering|Material|SetMaterial (Variables|Default|GetStaticMesh) 1 (select (Variables|Default|GetIsPrimary) "/Game/Superliminal/Assets/Materials/MI_Portal1.MI_Portal1" "/Game/Superliminal/Assets/Materials/MI_Portal0.MI_Portal0")))

(fn UpdateRenerTarget
  (bind _returnvalue (Viewport|GetViewportSize))
  (bind _mirror (Variables|Default|GetMirror))
  (bind _as_bp_superliminal_character (Variables|Default|GetAs%20BP%20Superliminal%20Character))
  (bind _returnvalue_2 (Transformation|GetWorldTransform _mirror))
  (bind _firstpersoncamera (Variables|/Game/FirstPerson/Blueprints/BP_FirstPersonCharacter.BP_FirstPersonCharacter_C|GetFirstPersonCamera _as_bp_superliminal_character))
  (bind _returnvalue_3 (Transformation|GetWorldTransform _firstpersoncamera))
  (bind _returnvalue_4 (Math|Transform|MakeRelativeTransform _returnvalue_3 _returnvalue_2))
  (Rendering|ResizeRenderTarget2D (Variables|/Script/Engine.SceneCaptureComponent2D|GetTextureTarget (Variables|Default|GetSceneCaptureComponent2D)) (Math|Float|Truncate (.x _returnvalue)) (Math|Float|Truncate (.y _returnvalue)))
  (Transformation|SetRelativeLocationAndRotation (Variables|BP_MoveableTeleport_C|GetSceneCaptureComponent2D (Variables|Default|GetLinkedPortal)) (.location _returnvalue_4) (.rotation _returnvalue_4) false false)
  (Variables|/Script/Engine.SceneCaptureComponent2D|SetClipPlaneBase (Variables|Default|GetSceneCaptureComponent2D) (Transformation|GetWorldLocation (Variables|Default|GetStaticMesh)))
  (Variables|/Script/Engine.SceneCaptureComponent2D|SetClipPlaneNormal (Variables|Default|GetSceneCaptureComponent2D) (Math|Vector|GetForwardVector (Variables|Default|GetStaticMesh)))
  (if (Variables|Default|GetStartOverlap)
    (if true
      (CallFunction|Teleport))))

(fn Teleport
  (LocalVariables|SetLVelocity (Math|Transform|TransformDirection (Transformation|GetWorldTransform (Variables|BP_MoveableTeleport_C|GetMirror (Variables|Default|GetLinkedPortal))) (Math|Transform|InverseTransformDirection (Transformation|GetWorldTransform (Variables|Default|GetStaticMesh)) (Transformation|GetVelocity (Variables|Default|GetAs%20BP%20Superliminal%20Character)))))
  (LocalVariables|SetLLocation (Math|Transform|TransformLocation (Transformation|GetWorldTransform (Variables|BP_MoveableTeleport_C|GetMirror (Variables|Default|GetLinkedPortal))) (Math|Transform|InverseTransformLocation (Transformation|GetWorldTransform (Variables|Default|GetStaticMesh)) (Transformation|GetActorLocation (Variables|Default|GetAs%20BP%20Superliminal%20Character)))))
  (LocalVariables|SetLRotation (Math|Transform|TransformRotation (Transformation|GetWorldTransform (Variables|BP_MoveableTeleport_C|GetMirror (Variables|Default|GetLinkedPortal))) (Math|Transform|InverseTransformRotation (Transformation|GetWorldTransform (Variables|Default|GetStaticMesh)) (Pawn|GetControlRotation (Pawn|GetController (Variables|Default|GetAs%20BP%20Superliminal%20Character)) :!class /Script/Engine.Controller))))
  (Pawn|SetControlRotation (Pawn|GetController (Variables|Default|GetAs%20BP%20Superliminal%20Character)) (LocalVariables|GetLRotation))
  (Default|ResizePlayerAfterTeleport (Variables|Default|GetAs%20BP%20Superliminal%20Character) (/ (.z (Transformation|GetWorldScale (Variables|/Game/Superliminal/Blueprints/Movable/BP_Moveable.BP_Moveable_C|GetStaticMesh (Variables|Default|GetLinkedPortal)))) (.x (Transformation|GetWorldScale (Variables|Default|GetStaticMesh)))))
  (Transformation|SetActorLocationAndRotation (Variables|Default|GetAs%20BP%20Superliminal%20Character) (LocalVariables|GetLLocation))
  (Variables|/Script/Engine.MovementComponent|SetVelocity (Variables|/Script/Engine.Character|GetCharacterMovement (Variables|Default|GetAs%20BP%20Superliminal%20Character)) (LocalVariables|GetLVelocity)))

(fn IsPlayerInfront
  (return (>= (Math|Vector|DotProduct (Math|Vector|GetForwardVector (Variables|Default|GetStaticMesh)) (Math|Vector|Normalize (- (Transformation|GetActorLocation (Variables|Default|GetAs%20BP%20Superliminal%20Character)) (Transformation|GetWorldLocation (Variables|Default|GetStaticMesh))))) 0.0)))